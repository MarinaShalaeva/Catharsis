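; BP_VictoryFirework is a victory effect actor that plays a Niagara firework with repeated sound.
; On BeginPlay it spawns the firework system at its location and starts a looping timer that triggers the sound through MulticastSpawnSound.
; The timer is cleared when the system finishes, is found invalid or inactive, or the play counter reaches its cap.
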(event `self.ReceiveBeginPlay`
  (bind _returnvalue (`NiagaraFunctionLibrary.SpawnSystemAtLocation` (`self.NS_Firework`) (`self.K2_GetActorLocation`)))
  (bind _output_get (set `self.SpawnedNiagara` _returnvalue))
  (add `NiagaraComponent.OnSystemFinished` _output_get (delegate `OnSystemFinished_Event`))
  (bind _returnvalue_2 (`KismetSystemLibrary.K2_SetTimerDelegate` (delegate `SpawnSound`) 2.0 true))
  (set `self.TH_SpawnSound` _returnvalue_2))

(event `OnSystemFinished_Event`
  (params (PSystem :type "NiagaraComponent Object Reference"))
  (bind _th_spawnsound (`self.TH_SpawnSound`))
  (if (`KismetSystemLibrary.K2_IsValidTimerHandle` _th_spawnsound)
    (`KismetSystemLibrary.K2_ClearAndInvalidateTimerHandle` _th_spawnsound)))

(event `SpawnSound`
  (`self.MulticastSpawnSound`))

(event `MulticastSpawnSound`
  (bind _th_spawnsound (`self.TH_SpawnSound`))
  (`/Engine/EditorBlueprintResources/StandardMacros.IncrementInt` (`self.FireworksCounter`)
    (:`  `
      (if (and (`KismetSystemLibrary.IsValid` (`self.SpawnedNiagara`)) (`ActorComponent.IsActive` (`self.SpawnedNiagara`)))
        (`AudioComponent.Play` (`self.FireworkSound`) 0.0)
        (if (== (`self.FireworksCounter`) 5)
          (if (`KismetSystemLibrary.K2_IsValidTimerHandle` _th_spawnsound) :!label _label
            (`KismetSystemLibrary.K2_ClearAndInvalidateTimerHandle` _th_spawnsound)))
        (else
          (goto _label))))))

(fn `UserConstructionScript`)
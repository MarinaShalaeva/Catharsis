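; BP_Sky is a sky actor that shows one of several sky materials on an inverted-normals sphere mesh.
; On BeginPlay it reads the current sky material index from CPP_GameState, applies it, and binds to the game state's change-sky-material event dispatcher.
; Each change swaps the sphere's material to the matching entry in its Materials array, if that entry is valid.
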(event `self.ReceiveBeginPlay`
  (bind _ascpp_game_state (cast `CPP_GameState` (`GameplayStatics.GetGameState`)))
  (`self.ChangeSkyMaterial` (`CPP_GameState.GetSkyMaterialIndex` _ascpp_game_state))
  (add `CPP_GameState.ED_ChangeSkyMaterial` _ascpp_game_state (delegate `ChangeSkyMaterial`)))

(event `ChangeSkyMaterial`
  (params (NewMaterialIndex :type Integer))
  (bind _output (`|GetArrayItem` (`self.Materials`) NewMaterialIndex))
  (`/Engine/EditorBlueprintResources/StandardMacros.IsValid` _output
    (:`Is Valid`
      (`PrimitiveComponent.SetMaterial` (`self.Sphere_inversenormals`) 0 _output))))

(fn `UserConstructionScript`)
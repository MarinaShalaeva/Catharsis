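; Player cat character Blueprint for the platformer, handling a damage screen effect and the cat's sounds.
; On BeginPlay it puts a dynamic damage post-process material on FollowCamera, reusing settings from a level PostProcessVolume.
; Two timelines drive that material's Intensity when the effect toggles.
; PlaySound maps sound types to audio components; walk and run share one movement component, swapping cues by surface and raising pitch for running.
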(event `self.ReceiveBeginPlay`
  (`self.InitPostProcessDamageMaterial`))

(event `self.ChangeEnablingOfPostProcessDamageMaterial`
  (params (bTurnOn :type Boolean))
  (if bTurnOn
    (`self.SetPostProcessDamageMaterial`)
    (else
      (`self.ResetPostProcessDamageMaterial`))))

(event `SetPostProcessDamageMaterial`
  (bind (_direction _intensity_track) (`Timeline|TL_TurnOn` :!via `PlayFromStart`)
    (:`Update`
      (`MaterialInstanceDynamic.SetScalarParameterValue` (`self.PP_Material`) "Intensity" _intensity_track))))

(event `ResetPostProcessDamageMaterial`
  (bind (_direction _intensity_track) (`Timeline|TL_TurnOff` :!via `PlayFromStart`)
    (:`Update`
      (`MaterialInstanceDynamic.SetScalarParameterValue` (`self.PP_Material`) "Intensity" _intensity_track))))

(event `self.PlaySound`
  (params (CatSound :type "ECatSoundState Enum" :default "None"))
  (switch `ECatSoundState` CatSound
    (:`None`
      (`self.StopPlayingAllSounds`))
    (:`BasicWalk`
      (`self.StartBasicWalkSound`))
    (:`BasicRun`
      (`self.StartBasicRunSound`))
    (:`GrassWalk`
      (`self.StartGrassWalkSound`))
    (:`GrassRun`
      (`self.StartGrassRunSound`))
    (:`Hiss`
      (`self.StartPlayingSound` (`self.HissSoundComponent`)))
    (:`Attack`
      (`self.StartPlayingSound` (`self.AttackSoundComponent`)))
    (:`HitGround`
      (`self.StartPlayingSound` (`self.HitTheGroundSoundComponent`)))))

(event `self.StopAllMovementSounds`
  (`AudioComponent.Stop` (`self.MovementSoundComponent`)))

(fn `InitPostProcessDamageMaterial`
  (bind _returnvalue (`KismetMaterialLibrary.CreateDynamicMaterialInstance` "/Game/CatPlatformer/PostProcess/MI_PostProcessDamage.MI_PostProcessDamage"))
  (set `self.PP_Material` _returnvalue)
  (bind _returnvalue_2 (`GameplayStatics.GetActorOfClass` "/Script/Engine.PostProcessVolume"))
  (`/Engine/EditorBlueprintResources/StandardMacros.IsValid` _returnvalue_2
    (:`Is Valid`
      (set `self.PP_DamageSettings` (`PostProcessVolume.Settings` _returnvalue_2)))
    (:`Is Not Valid`
      _))
  (bind _structout (setmembers `PostProcessSettings` :`StructRef` (`self.PP_DamageSettings`) :`WeightedBlendables` (make `WeightedBlendables` (`|MakeArray` (make `WeightedBlendable` 1.0 (`self.PP_Material`))))))
  (set `CameraComponent.PostProcessSettings` _structout (`self.FollowCamera`)))

(fn `StartBasicRunSound`
  (bind _movementsoundcomponent (`self.MovementSoundComponent`))
  (if (!= (`AudioComponent.Sound` (`self.MovementSoundComponent`)) "/Game/CatPlatformer/Sounds/SFX/Cat/CatCarpetWalk_Sound_Cue.CatCarpetWalk_Sound_Cue")
    (`AudioComponent.SetSound` _movementsoundcomponent "/Game/CatPlatformer/Sounds/SFX/Cat/CatCarpetWalk_Sound_Cue.CatCarpetWalk_Sound_Cue"))
  (`AudioComponent.SetPitchMultiplier` _movementsoundcomponent 1.31)
  (if (not (`AudioComponent.IsPlaying` (`self.MovementSoundComponent`)))
    (`self.StartPlayingSound` _movementsoundcomponent)))

(fn `StartBasicWalkSound`
  (bind _movementsoundcomponent (`self.MovementSoundComponent`))
  (if (!= (`AudioComponent.Sound` (`self.MovementSoundComponent`)) "/Game/CatPlatformer/Sounds/SFX/Cat/CatCarpetWalk_Sound_Cue.CatCarpetWalk_Sound_Cue")
    (`AudioComponent.SetSound` _movementsoundcomponent "/Game/CatPlatformer/Sounds/SFX/Cat/CatCarpetWalk_Sound_Cue.CatCarpetWalk_Sound_Cue"))
  (`AudioComponent.SetPitchMultiplier` _movementsoundcomponent 1.0)
  (if (not (`AudioComponent.IsPlaying` (`self.MovementSoundComponent`)))
    (`self.StartPlayingSound` _movementsoundcomponent)))

(fn `StartGrassRunSound`
  (bind _movementsoundcomponent (`self.MovementSoundComponent`))
  (if (!= (`AudioComponent.Sound` (`self.MovementSoundComponent`)) "/Game/CatPlatformer/Sounds/SFX/Cat/CatWalkGrass_Sound_Cue.CatWalkGrass_Sound_Cue")
    (`AudioComponent.SetSound` _movementsoundcomponent "/Game/CatPlatformer/Sounds/SFX/Cat/CatWalkGrass_Sound_Cue.CatWalkGrass_Sound_Cue"))
  (`AudioComponent.SetPitchMultiplier` _movementsoundcomponent 1.35)
  (if (not (`AudioComponent.IsPlaying` (`self.MovementSoundComponent`)))
    (`self.StartPlayingSound` _movementsoundcomponent)))

(fn `StartGrassWalkSound`
  (bind _movementsoundcomponent (`self.MovementSoundComponent`))
  (if (!= (`AudioComponent.Sound` (`self.MovementSoundComponent`)) "/Game/CatPlatformer/Sounds/SFX/Cat/CatWalkGrass_Sound_Cue.CatWalkGrass_Sound_Cue")
    (`AudioComponent.SetSound` _movementsoundcomponent "/Game/CatPlatformer/Sounds/SFX/Cat/CatWalkGrass_Sound_Cue.CatWalkGrass_Sound_Cue"))
  (`AudioComponent.SetPitchMultiplier` _movementsoundcomponent 1.0)
  (if (not (`AudioComponent.IsPlaying` (`self.MovementSoundComponent`)))
    (`self.StartPlayingSound` _movementsoundcomponent)))

(fn `StartPlayingSound`
  (params (Sound :type "AudioComponent Object Reference"))
  (`AudioComponent.Play` Sound 0.0))

(fn `StopPlayingAllSounds`
  (`self.StopPlayingSound` (`self.MovementSoundComponent`))
  (`self.StopPlayingSound` (`self.HissSoundComponent`))
  (`self.StopPlayingSound` (`self.AttackSoundComponent`))
  (`self.StopPlayingSound` (`self.HitTheGroundSoundComponent`)))

(fn `StopPlayingSound`
  (params (Sound :type "AudioComponent Object Reference"))
  (if (`AudioComponent.IsPlaying` Sound)
    (`AudioComponent.Stop` Sound))
  (if (== Sound (`self.MovementSoundComponent`))
    (`AudioComponent.SetSound` (`self.MovementSoundComponent`) null)))

(fn `UserConstructionScript`)